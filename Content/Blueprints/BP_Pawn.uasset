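; BP_Pawn is a pawn that runs a gaze check to detect which cube the camera is looking at.
; Every tick it fires a debug-drawn visibility line trace forward from the camera.
; The hit actor is cast to BP_Cube, then to BP_BlueCube, printing a red or blue "found" message on screen.
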(event `self.ReceiveTick`
  (params (DeltaSeconds :type "Float (single-precision)"))
  (`self.GazeCheck`))

(event `GazeCheck`
  (bind _camera (`self.Camera`))
  (bind _returnvalue (`SceneComponent.K2_GetComponentLocation` _camera))
  ;[1 1 1] Gaze Check
  (bind _outhit (`KismetSystemLibrary.LineTraceSingle` :`Start` _returnvalue :`End` (+ _returnvalue (* (`SceneComponent.GetForwardVector` _camera) 2000.0)) :`TraceChannel` "TraceTypeQuery1" :`DrawDebugType` "ForOneFrame" :`TraceColor` (struct :`R` 1.0 :`G` 1.0 :`B` 1.0 :`A` 1.0)))
  (bind (_bblockinghit _binitialoverlap _time _location _impactpoint _normal _impactnormal _physmat _hitactor) (`GameplayStatics.BreakHitResult` _outhit))
  (cast `/Game/Blueprints/BP_Cube` _hitactor
    (:`then`
      (`KismetSystemLibrary.PrintString` "Found Red" true true (struct :`R` 1.0 :`B` 0.213813 :`A` 1.0)))
    (:`CastFailed`
      (cast `/Game/Blueprints/BP_BlueCube` _hitactor)
      (`KismetSystemLibrary.PrintString` "Found Blue"))))

(fn `UserConstructionScript`)